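; BP_Visitor is a visitor actor that wanders randomly across a tile grid until it is removed.
; When idle, it checks the four neighboring cells for two allowed cell states and picks one at random as its next target.
; Tick moves it toward that tile at constant speed, clamping the last step.
; Reaching a cell of the removal state decrements the Spawner's visitor count and destroys the actor.
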(event EventBeginPlay)

(event Collision|EventActorBeginOverlap
  (params (OtherActor :type Actor%20Object%20Reference)))

(event EventTick
  (params (DeltaSeconds :type Float%20%28single-precision%29))
  (bind _spawner (Variables|Default|GetSpawner))
  (if (!= (Variables|Default|GetisMoving) true)
    (if (Variables|Default|GetRemoveAfterMove)
      (Variables|/Game/Progger/Markus/GridSystem/VisitorSpawner.VisitorSpawner_C|SetCurrentVisitorCount _spawner (- (Variables|/Game/Progger/Markus/GridSystem/VisitorSpawner.VisitorSpawner_C|GetCurrentVisitorCount _spawner) 1))
      (Actor|DestroyActor)
      (else
        (bind (_movedirection _succes) (CallFunction|GetMoveDirection))
        (if _succes
          (CallFunction|Moveto _movedirection))))
    (else
      (CallFunction|MoveTick DeltaSeconds))))

(fn ConstructionScript)

(fn Moveto
  (params (MovePosition :type Vector))
  (Variables|Default|SetStartPosition MovePosition)
  (Variables|Default|SetisMoving true)
  (Variables|Default|SetGoalTransform (Math|Transform|MakeTransform (+ (* (Variables|/Game/Progger/Markus/GridSystem/Grid.Grid_C|GetTileSize (Variables|Default|GetGrid)) MovePosition) (Math|Vector|MakeVector 0.0 0.0 (.z (.location (Transformation|GetActorTransform))))) "0, 0, 0" "1.000000,1.000000,1.000000")))

(fn MoveTick
  (params (TickDelta :type Float%20%28double-precision%29))
  (bind _returnvalue (Transformation|GetActorTransform))
  (bind _speed (Variables|Default|GetSpeed))
  (bind _goaltransform (Variables|Default|GetGoalTransform))
  (bind _returnvalue_2 (- (.location _goaltransform) (.location _returnvalue)))
  (bind _returnvalue_3 (Math|Vector|Normalize _returnvalue_2))
  (bind _returnvalue_4 (* _returnvalue_3 _speed TickDelta))
  (if (> (Math|Vector|VectorLength _returnvalue_4) (Math|Vector|VectorLength _returnvalue_2))
    (LocalVariables|SetMoveDistance _returnvalue_2)
    (Variables|Default|SetisMoving false)
    (else
      (LocalVariables|SetMoveDistance _returnvalue_4)))
  (Class|Actor|AddActorWorldTransform (Math|Transform|MakeTransform (LocalVariables|GetMoveDistance) "0, 0, 0" "1.000000,1.000000,1.000000") false false))

(fn GetMoveDirection
  (bind _wayinfo (LocalVariables|GetWayInfo))
  (bind _returnvalue (Utilities|Array|IsNotEmpty _wayinfo))
  (bind _cellinformation (Default|GetCellInformation (Variables|Default|GetGrid) (+ (Variables|Default|GetStartPosition) "0.000000,1.000000,0.000000")))
  (if (or (Utilities|Enum|Equal(Enum) (.cellstate _cellinformation) "NewEnumerator2") (Utilities|Enum|Equal(Enum) (.cellstate _cellinformation) "NewEnumerator5"))
    (Utilities|Array|Add (LocalVariables|GetWayInfo) (.position _cellinformation)))
  (bind _cellinformation_2 (Default|GetCellInformation (Variables|Default|GetGrid) (+ (Variables|Default|GetStartPosition) "1.000000,0.000000,0.000000")))
  (if (or (Utilities|Enum|Equal(Enum) (.cellstate _cellinformation_2) "NewEnumerator2") (Utilities|Enum|Equal(Enum) (.cellstate _cellinformation_2) "NewEnumerator5"))
    (Utilities|Array|Add (LocalVariables|GetWayInfo) (.position _cellinformation_2)))
  (bind _cellinformation_3 (Default|GetCellInformation (Variables|Default|GetGrid) (+ (Variables|Default|GetStartPosition) "0.000000,-1.000000,0.000000")))
  (if (or (Utilities|Enum|Equal(Enum) (.cellstate _cellinformation_3) "NewEnumerator2") (Utilities|Enum|Equal(Enum) (.cellstate _cellinformation_3) "NewEnumerator5"))
    (Utilities|Array|Add (LocalVariables|GetWayInfo) (.position _cellinformation_3)))
  (bind _cellinformation_4 (Default|GetCellInformation (Variables|Default|GetGrid) (+ (Variables|Default|GetStartPosition) "-1.000000,0.000000,0.000000")))
  (if (or (Utilities|Enum|Equal(Enum) (.cellstate _cellinformation_4) "NewEnumerator2") (Utilities|Enum|Equal(Enum) (.cellstate _cellinformation_4) "NewEnumerator5"))
    (Utilities|Array|Add (LocalVariables|GetWayInfo) (.position _cellinformation_4)))
  (LocalVariables|SetSuccesState _returnvalue)
  (if _returnvalue
    (bind _output_get (LocalVariables|SetOutput (.OutItem (Utilities|Array|Random (LocalVariables|GetWayInfo)))))
    (bind _cellinformation_5 (Default|GetCellInformation (Variables|Default|GetGrid) _output_get))
    (if (Utilities|Enum|Equal(Enum) (.cellstate _cellinformation_5) "NewEnumerator5")
      (Variables|Default|SetRemoveAfterMove true)))
  (return (LocalVariables|GetOutput) (LocalVariables|GetSuccesState)))