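; Main-menu scene Blueprint that plays a sound on BeginPlay, creates quit, settings and credits widgets collapsed, then shows the main menu and mouse cursor.
; Its timed three-logo intro sits behind a constant-true branch and never runs, as the game instance's WasAlreadyInGame read is unused.
; WidgetArray serves as a navigation stack: helper functions push, collapse or reset menus, MenuUp returns to the previous one, and EqualMenu is empty.
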(event EventBeginPlay
  (Audio|PlaySound2D 0 1.0 1.0 0.0 0 0)
  (bind _asbp_game_instance (Utilities|Casting|CastToBP_GameInstance (Game|GetGameInstance)))
  (if true
    _
    (else
      (Variables|/Game/Julian/Blueprints/BP_GameInstance.BP_GameInstance_C|SetwasAlreadyInGame _asbp_game_instance true)
      (bind _returnvalue (UserInterface|CreateWidget "/Game/Julian/Widgets/WB_Logo_GA.WB_Logo_GA_C"))
      (bind _output_get (Variables|Default|SetLoadingScreenGA _returnvalue))
      (UserInterface|Viewport|AddtoViewport _output_get 0)
      (bind _returnvalue_2 (UserInterface|CreateWidget "/Game/Julian/Widgets/WB_Logo_Team.WB_Logo_Team_C"))
      (bind _output_get_2 (Variables|Default|SetLoadingScreenTeamLogo _returnvalue_2))
      (UserInterface|Viewport|AddtoViewport _output_get_2 0)
      (bind _returnvalue_3 (UserInterface|CreateWidget "/Game/Julian/Widgets/WB_Logo_Game.WB_Logo_Game_C"))
      (bind _output_get_3 (Variables|Default|SetFantasticMenagerieLogo _returnvalue_3))
      (UserInterface|Viewport|AddtoViewport _output_get_3 0)
      (Utilities|FlowControl|Delay 4.0)
      (Widget|RemovefromParent (Variables|Default|GetFantasticMenagerieLogo))
      (Utilities|FlowControl|Delay 4.0)
      (Widget|RemovefromParent (Variables|Default|GetLoadingScreenTeamLogo))
      (Utilities|FlowControl|Delay 4.0)
      (Widget|RemovefromParent (Variables|Default|GetLoadingScreenGA))))
  (bind _returnvalue_4 (UserInterface|CreateWidget "/Game/Julian/Widgets/WB_Quit.WB_Quit_C"))
  (bind _output_get_4 (Variables|Default|SetQuit _returnvalue_4))
  (UserInterface|Viewport|AddtoViewport _output_get_4 0)
  (Variables|/Script/UMG.Widget|SetVisibility _output_get_4 "Collapsed")
  (bind _returnvalue_5 (UserInterface|CreateWidget "/Game/Julian/Widgets/WB_Settings.WB_Settings_C"))
  (bind _output_get_5 (Variables|Default|SetAudioSettings _returnvalue_5))
  (UserInterface|Viewport|AddtoViewport _output_get_5 0)
  (Variables|/Script/UMG.Widget|SetVisibility (Variables|Default|GetAudioSettings) "Collapsed")
  (bind _returnvalue_6 (UserInterface|CreateWidget "/Game/Julian/Widgets/WB_Credits.WB_Credits_C"))
  (bind _output_get_6 (Variables|Default|SetCredits _returnvalue_6))
  (UserInterface|Viewport|AddtoViewport _output_get_6 0)
  (Variables|/Script/UMG.Widget|SetVisibility (Variables|Default|GetCredits) "Collapsed")
  (Variables|/Script/Engine.PlayerController|SetbShowMouseCursor (Game|GetPlayerController 0) true)
  (bind _returnvalue_7 (UserInterface|CreateWidget "/Game/Julian/Widgets/WB_MainMenu.WB_MainMenu_C"))
  (bind _output_get_7 (Variables|Default|SetMainMenu _returnvalue_7))
  (UserInterface|Viewport|AddtoViewport _output_get_7 0)
  (Utilities|Array|Add (Variables|Default|GetWidgetArray) _output_get_7))

(fn ConstructionScript)

(fn SubMenuOpen
  (params (WidgetToOpen :type User%20Widget%20Object%20Reference))
  (Utilities|Array|Add (Variables|Default|GetWidgetArray) WidgetToOpen)
  (Variables|/Script/UMG.Widget|SetVisibility WidgetToOpen "Visible"))

(fn SubMenuClosed
  (params (WidgetToOpen :type User%20Widget%20Object%20Reference))
  (bind _widgetarray (Variables|Default|GetWidgetArray))
  (for _array_element _widgetarray
    (Variables|/Script/UMG.Widget|SetVisibility _array_element "Collapsed"))
  (Utilities|Array|Add _widgetarray WidgetToOpen)
  (Variables|/Script/UMG.Widget|SetVisibility WidgetToOpen "Visible"))

(fn EqualMenu)

(fn AlphaMenu
  (params (WidgetToOpen :type User%20Widget%20Object%20Reference))
  (bind _widgetarray (Variables|Default|GetWidgetArray))
  (for _array_element _widgetarray
    (Variables|/Script/UMG.Widget|SetVisibility _array_element "Collapsed"))
  (Utilities|Array|Clear _widgetarray)
  (Utilities|Array|Add _widgetarray WidgetToOpen)
  (Variables|/Script/UMG.Widget|SetVisibility WidgetToOpen "Visible"))

(fn MenuUp
  (bind _widgetarray (Variables|Default|GetWidgetArray))
  (bind _returnvalue (Utilities|Array|LastIndex _widgetarray))
  (bind _output (Utilities|Array|Get(acopy) _widgetarray _returnvalue))
  (Variables|/Script/UMG.Widget|SetVisibility _output "Collapsed")
  (Utilities|Array|RemoveIndex _widgetarray _returnvalue)
  (Variables|/Script/UMG.Widget|SetVisibility _output "Visible"))