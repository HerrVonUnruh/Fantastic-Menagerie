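; Gameplay manager that boots the level's UI and soundtrack and handles menu navigation.
; BeginPlay hides the BP_Grid actor, shows a timed loading screen, and pre-creates the HUD, build and menu widgets collapsed, seeding starting cashflow.
; WidgetArray acts as a menu stack: helpers push a submenu with or without hiding others, pop back, or reset to one root menu.
; EqualMenu is an empty stub, and the FPS widget setup never runs.
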(event EventBeginPlay
  (bind _returnvalue (Actor|GetActorOfClass "/Game/Robin/NewLevel/Blueprint/Grid/BP_Grid.BP_Grid_C"))
  (bind _output_get (Variables|Default|SetGrid _returnvalue))
  (Rendering|SetActorHiddenInGame _output_get true)
  (if true
    (bind _returnvalue_2 (UserInterface|CreateWidget "/Game/Julian/Widgets/WB_Loadingscreen.WB_Loadingscreen_C"))
    (UserInterface|Viewport|AddtoViewport _returnvalue_2 0))
  (Variables|Default|SetGameSpeed 1.0)
  (Utilities|FlowControl|Delay 0.2)
  (Audio|PlaySound2D "/Game/SoundDesign/OSTs/Fantastic_Beatszoo_Gameplay_soundtrack_Final_Version.Fantastic_Beatszoo_Gameplay_soundtrack_Final_Version" 1.0 1.0 0.0 0 0)
  (bind _returnvalue_3 (UserInterface|CreateWidget "/Game/Julian/Widgets/WB_BacktoMainMenu.WB_BacktoMainMenu_C"))
  (bind _output_get_2 (Variables|Default|SetBackToMainMenu _returnvalue_3))
  (UserInterface|Viewport|AddtoViewport _output_get_2 0)
  (Variables|/Script/UMG.Widget|SetVisibility _output_get_2 "Collapsed")
  (bind _returnvalue_4 (UserInterface|CreateWidget "/Game/Julian/Widgets/WB_Quit.WB_Quit_C"))
  (bind _output_get_3 (Variables|Default|SetQuit _returnvalue_4))
  (UserInterface|Viewport|AddtoViewport _output_get_3 0)
  (Variables|/Script/UMG.Widget|SetVisibility _output_get_3 "Collapsed")
  (bind _returnvalue_5 (UserInterface|CreateWidget "/Game/Julian/Widgets/WB_Settings.WB_Settings_C"))
  (bind _output_get_4 (Variables|Default|SetAudio%20Settings _returnvalue_5))
  (UserInterface|Viewport|AddtoViewport _output_get_4 0)
  (Variables|/Script/UMG.Widget|SetVisibility (Variables|Default|GetAudio%20Settings) "Collapsed")
  (bind _returnvalue_6 (UserInterface|CreateWidget "/Game/Julian/Widgets/WB_Credits.WB_Credits_C"))
  (bind _output_get_5 (Variables|Default|SetCredits _returnvalue_6))
  (UserInterface|Viewport|AddtoViewport _output_get_5 0)
  (Variables|/Script/UMG.Widget|SetVisibility (Variables|Default|GetCredits) "Collapsed")
  (bind _returnvalue_7 (UserInterface|CreateWidget "/Game/Julian/Widgets/WB_Controls.WB_Controls_C"))
  (bind _output_get_6 (Variables|Default|SetControls _returnvalue_7))
  (UserInterface|Viewport|AddtoViewport _output_get_6 0)
  (Variables|/Script/UMG.Widget|SetVisibility (Variables|Default|GetControls) "Collapsed")
  (bind _returnvalue_8 (UserInterface|CreateWidget "/Game/Julian/Widgets/WB_BuildMenu.WB_BuildMenu_C"))
  (bind _output_get_7 (Variables|Default|SetBau%20Menu _returnvalue_8))
  (UserInterface|Viewport|AddtoViewport _output_get_7 0)
  (Variables|/Script/UMG.Widget|SetVisibility (Variables|Default|GetBau%20Menu) "Collapsed")
  (bind _returnvalue_9 (UserInterface|CreateWidget "/Game/Julian/Widgets/WB_CoreInterface.WB_CoreInterface_C"))
  (Default|CashflowFunction _returnvalue_9 1500)
  (bind _output_get_8 (Variables|Default|SetCoreInterface _returnvalue_9))
  (UserInterface|Viewport|AddtoViewport _output_get_8 0)
  (Variables|/Script/UMG.Widget|SetVisibility (Variables|Default|GetCoreInterface) "Collapsed")
  (bind _returnvalue_10 (UserInterface|CreateWidget "/Game/Julian/Widgets/WB_IngameMenu.WB_IngameMenu_C"))
  (bind _output_get_9 (Variables|Default|SetIngame%20Menu _returnvalue_10))
  (UserInterface|Viewport|AddtoViewport _output_get_9 0)
  (Variables|/Script/UMG.Widget|SetVisibility (Variables|Default|GetIngame%20Menu) "Collapsed")
  (Utilities|FlowControl|Delay 3.0)
  (Utilities|IsValid _returnvalue_2
    (:Is%20Valid
      (Widget|RemovefromParent _returnvalue_2))
    (:Is%20Not%20Valid
      _))
  (Variables|/Script/UMG.Widget|SetVisibility (Variables|Default|GetCoreInterface) "Collapsed"))

(fn ConstructionScript)

(fn SubMenuClosed
  (params (WidgetToOpen :type User%20Widget%20Object%20Reference))
  (bind _widgetarray (Variables|Default|GetWidgetArray))
  (for _array_element _widgetarray
    (Variables|/Script/UMG.Widget|SetVisibility _array_element "Collapsed"))
  (Utilities|Array|Add _widgetarray WidgetToOpen)
  (Variables|/Script/UMG.Widget|SetVisibility WidgetToOpen "Visible"))

(fn SubMenuOpen
  (params (WidgetToOpen :type User%20Widget%20Object%20Reference))
  (Utilities|Array|Add (Variables|Default|GetWidgetArray) WidgetToOpen)
  (Variables|/Script/UMG.Widget|SetVisibility WidgetToOpen "Visible"))

(fn MenuUp
  (bind _widgetarray (Variables|Default|GetWidgetArray))
  (bind _returnvalue (Utilities|Array|LastIndex _widgetarray))
  (bind _output (Utilities|Array|Get(acopy) _widgetarray _returnvalue))
  (Variables|/Script/UMG.Widget|SetVisibility _output "Collapsed")
  (Utilities|Array|RemoveIndex _widgetarray _returnvalue)
  (if (Utilities|Array|IsNotEmpty _widgetarray)
    (Variables|/Script/UMG.Widget|SetVisibility _output "Visible")))

(fn AlphaMenu
  (params (WidgetToOpen :type User%20Widget%20Object%20Reference))
  (bind _widgetarray (Variables|Default|GetWidgetArray))
  (for _array_element _widgetarray
    (Variables|/Script/UMG.Widget|SetVisibility _array_element "Collapsed"))
  (Utilities|Array|Clear _widgetarray)
  (Utilities|Array|Add _widgetarray WidgetToOpen)
  (Variables|/Script/UMG.Widget|SetVisibility WidgetToOpen "Visible"))

(fn EqualMenu
  (params (WidgetToOpen :type User%20Widget%20Object%20Reference)))