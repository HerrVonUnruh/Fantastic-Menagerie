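; Base grid unit, either character or building, whose meshes and animation class come from its unit type's data at construction.
; Follows tile paths recursively with a rate-scaled timeline, lerping position and yaw, adding a jump offset across height changes, and broadcasting tile-reached and walk-finished events.
; Sends idle/walk states to the AnimInstance by message and tints the skeletal mesh for hover and selection.
; Holds a grid reference and attaches an assigned AI actor.
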(event Custom|Event_FollowPath
  (params (Path :type Array%20of%20Int%20Point%20Structures))
  (if (> (Utilities|Array|Length Path) 0)
    (Variables|Default|SetCurrentPathToFollow Path)
    (CallFunction|ContinuetoFollowPath)))

(event Custom|ContinueToFollowPath
  (bind _grid (Variables|Default|GetGrid))
  (bind _currentpathtofollow (Variables|Default|GetCurrentPathToFollow))
  (bind _timeline_unitmovement (Variables|Default|GetTimeline_UnitMovement))
  (bind _output (Utilities|Array|Get(acopy) _currentpathtofollow))
  (bind _gridtiles (Variables|/Game/Robin/NewLevel/Blueprint/Grid/BP_Grid.BP_Grid_C|GetGridTiles _grid))
  (bind _value (Utilities|Map|Find _gridtiles _output))
  (bind _transform (Utilities|Struct|BreakS_TileData _value))
  (if (> (Utilities|Array|Length (Variables|Default|GetCurrentPathToFollow)) 0)
    (CallFunction|SetAnimationState "NewEnumerator1")
    (Variables|Default|SetPreviousTransform (Transformation|GetActorTransform))
    (Variables|Default|SetNextTransform (Math|Transform|MakeTransform (.location _transform) (Math|Rotator|MakeRotator 0.0 0.0 (.yaw (Math|Rotator|FindLookatRotation (.location (Variables|Default|GetPreviousTransform)) (.location _transform)))) "1.000000,1.000000,1.000000"))
    (Components|Timeline|SetPlayRate _timeline_unitmovement (/ (Components|Timeline|GetTimelineLength _timeline_unitmovement) (Variables|Default|GetMoveDurationPerTile)))
    (bind (_direction _location_alpha _rotation_alpha _jump) (Timeline|Timeline_UnitMovement PlayFromStart)
      (:Update
        (Transformation|SetActorLocationAndRotation (+ (Math|Vector|Lerp(Vector) (.location (Variables|Default|GetPreviousTransform)) (.location (Variables|Default|GetNextTransform)) _location_alpha) (Math|Vector|MakeVector 0.0 0.0 (select (Math|Float|NearlyEqual(Float) (.z (.location (Variables|Default|GetPreviousTransform))) (.z (.location (Variables|Default|GetNextTransform))) 5.0) 0.0 _jump))) (Math|Rotator|Lerp(Rotator) (.rotation (Variables|Default|GetPreviousTransform)) (.rotation (Variables|Default|GetNextTransform)) _rotation_alpha true)))
      (:Finished
        (Default|CallOnUnitReachNewTile self (Utilities|Array|Get(acopy) (Variables|Default|GetCurrentPathToFollow)))
        (Utilities|Array|RemoveIndex (Variables|Default|GetCurrentPathToFollow))
        (CallFunction|ContinuetoFollowPath)))
    (else
      (CallFunction|SetAnimationState "NewEnumerator0")
      (Default|CallOnUnitFinishedWalking self))))

(event EventBeginPlay
  (CallFunction|SetAnimationState "NewEnumerator0"))

(fn ConstructionScript
  (bind _unitdata (CallFunction|GetDefaultUnitDatafromUnitType (Variables|Default|GetUnitType)))
  (CallFunction|SetUnitData _unitdata))

(fn UpdateVisualifHoveredorSelected
  (Rendering|Material|SetVectorParameterValueonMaterials (Variables|Default|GetSkeletalMesh) "ColorMultiply" (Math|Conversions|ToVector(LinearColor) (* (* (select (Variables|Default|GetIsSelected) "(R=0.130956,G=0.699575,B=0.866667,A=1.000000)" "(R=1.000000,G=1.000000,B=1.000000,A=1.000000)") (select (Variables|Default|GetIsHovered) 2.5 1.0)) (select (Variables|Default|GetIsSelected) 2.5 1.0)))))

(fn SetIsHovered
  (params (Hovered :type Boolean))
  (Variables|Default|SetIsHovered Hovered)
  (CallFunction|UpdateVisualifHoveredorSelected))

(fn SetIsSelected
  (params (Selected :type Boolean))
  (Variables|Default|SetIsSelected Selected)
  (CallFunction|UpdateVisualifHoveredorSelected))

(fn SetUnitData
  (params (Data :type S%20Unit%20Data%20Structure%20%28by%20ref%29))
  (bind _skeletalmesh (Variables|Default|GetSkeletalMesh))
  (bind _output_get (Variables|Default|SetUnitData Data))
  (if (.IsBuilding (Utilities|Struct|BreakS_UnitData_Assets (.Assets (Utilities|Struct|BreakS_UnitData _output_get))))
    (Components|StaticMesh|SetStaticMesh (Variables|Default|GetStaticMesh) (.StaticMesh (Utilities|Struct|BreakS_UnitData_Assets (.Assets (Utilities|Struct|BreakS_UnitData _output_get)))))
    (else
      (Variables|/Script/Engine.SkeletalMeshComponent|SetSkeletalMeshAsset _skeletalmesh (.Mesh (Utilities|Struct|BreakS_UnitData_Assets (.Assets (Utilities|Struct|BreakS_UnitData _output_get)))))))
  (Class|SkeletalMeshComponent|SetAnimClass _skeletalmesh (.AnimBp (Utilities|Struct|BreakS_UnitData_Assets (.Assets (Utilities|Struct|BreakS_UnitData _output_get))))))

(fn SetAnimationState
  (params (State :type E_UnitAnimationState%20Enum :default "NewEnumerator0"))
  (Class|BPIUnitAnimation|SetUnitAnimationState(Message) (Components|SkeletalMesh|GetAnimInstance (Variables|Default|GetSkeletalMesh)) State))

(fn SetGrid
  (params (Grid :type BP%20Grid%20Object%20Reference))
  (Variables|Default|SetGrid Grid))

(fn SetUnitAi
  (params (Ai :type BP%20Unit%20AI%20Object%20Reference))
  (bind _output_get (Variables|Default|SetAi Ai))
  (Utilities|IsValid _output_get
    (:Is%20Valid
      (Transformation|AttachActorToActor Ai self "None" "SnapToTarget" "SnapToTarget" "SnapToTarget" true))))