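; BP_BuildingSystem manages combat buildings on the tile grid, syncing each one's tile data and world location to its index.
; It listens for grid generation and tile updates, re-snapping buildings or destroying those on unwalkable tiles.
; Index changes update tile occupancy and fire a change event.
; Destroying credits money through the core UI; AddBuildingInCombat only deducts cost, as its registration and placement logic is disconnected.
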(event EventBeginPlay
  (bind _grid (Variables|Default|GetGrid))
  (EventDispatchers|BindEventtoOnGridGenerated _grid (EventDispatchers|CreateEvent :!event OnGridGenerated))
  (EventDispatchers|BindEventtoOnTileDataUpdated _grid (EventDispatchers|CreateEvent :!event OnTileDataUpdatet)))

(fn ConstructionScript)

(fn AddBuildinginCombat
  (params (Building :type BP%20Building%20Object%20Reference) (Index :type Int%20Point%20Structure))
  (bind _asbp_gm (Utilities|Casting|CastToBP_GM (Game|GetGameMode)))
  (bind _aswb_core_interface (Utilities|Casting|CastToWB_CoreInterface (Variables|/Game/Robin/NewLevel/Blueprint/Core/Player/BP_GM.BP_GM_C|GetCoreInterface _asbp_gm)))
  (Default|CashflowFunction _aswb_core_interface -150))

(fn RemoveBuildingfromCombat
  (params (Building :type BP%20Building%20Object%20Reference) (DestroyUnit :type Boolean))
  (Utilities|Array|RemoveItem (Variables|Default|GetBuilding) Building)
  (CallFunction|SetBuildingIndexonGrid Building (Utilities|Struct|MakeIntPoint -999 -999) false)
  (if DestroyUnit
    (Actor|DestroyActor Building)
    (bind _asbp_gm (Utilities|Casting|CastToBP_GM (Game|GetGameMode)))
    (bind _aswb_core_interface (Utilities|Casting|CastToWB_CoreInterface (Variables|/Game/Robin/NewLevel/Blueprint/Core/Player/BP_GM.BP_GM_C|GetCoreInterface _asbp_gm)))
    (Default|CashflowFunction _aswb_core_interface 100)))

(fn SetBuildingIndexonGrid
  (params (Building :type BP%20Building%20Object%20Reference) (Index :type Int%20Point%20Structure) (Force :type Boolean))
  (Utilities|FlowControl|Sequence
    (:then_0
      (if (or (!= (Variables|/Game/Robin/NewLevel/Blueprint/JulianUndRobin/BP_Building.BP_Building_C|GetIndex Building) Index) Force)
        (Utilities|FlowControl|Sequence
          (:then_0
            (bind _output_get (LocalVariables|SetPrevious%20Tile (.Value (Utilities|Map|Find (Variables|/Game/Robin/NewLevel/Blueprint/Grid/BP_Grid.BP_Grid_C|GetGridTiles (Variables|Default|GetGrid)) (Variables|/Game/Robin/NewLevel/Blueprint/JulianUndRobin/BP_Building.BP_Building_C|GetIndex Building)))))
            (if (== (.BuildingOnTile (Utilities|Struct|BreakS_TileData _output_get)) Building)
              (bind _structout (Utilities|Struct|SetmembersinS_TileData (LocalVariables|GetPrevious%20Tile) 0))
              (Utilities|Map|Add (Variables|/Game/Robin/NewLevel/Blueprint/Grid/BP_Grid.BP_Grid_C|GetGridTiles (Variables|Default|GetGrid)) (.Index (Utilities|Struct|BreakS_TileData _structout)) _structout)))
          (:then_1
            (Variables|/Game/Robin/NewLevel/Blueprint/JulianUndRobin/BP_Building.BP_Building_C|SetIndex Building Index)
            (if (!= Index (Utilities|Struct|MakeIntPoint -999 -999))
              (bind _structout_2 (Utilities|Struct|SetmembersinS_TileData (.Value (Utilities|Map|Find (Variables|/Game/Robin/NewLevel/Blueprint/Grid/BP_Grid.BP_Grid_C|GetGridTiles (Variables|Default|GetGrid)) Index)) Building))
              (Utilities|Map|Add (Variables|/Game/Robin/NewLevel/Blueprint/Grid/BP_Grid.BP_Grid_C|GetGridTiles (Variables|Default|GetGrid)) (.Index (Utilities|Struct|BreakS_TileData _structout_2)) _structout_2)))
          (:then_2
            (Default|CallOnBuildingGridIndexChanged Building)))))
    (:then_1
      (Transformation|SetActorLocation Building (select (.ReturnValue (Utilities|Map|Find (Variables|/Game/Robin/NewLevel/Blueprint/Grid/BP_Grid.BP_Grid_C|GetGridTiles (Variables|Default|GetGrid)) Index)) (.location (.Transform (Utilities|Struct|BreakS_TileData (.Value (Utilities|Map|Find (Variables|/Game/Robin/NewLevel/Blueprint/Grid/BP_Grid.BP_Grid_C|GetGridTiles (Variables|Default|GetGrid)) Index))))) "-99999.000000,-99999.000000,-99999.000000") false false))))

(fn OnGridGenerated
  (bind _output_get (LocalVariables|SetCopy%20Of%20Buildings (Variables|Default|GetBuilding)))
  (for _array_element _output_get
    (if (Default|IsTileWalkable (Variables|Default|GetGrid) (Variables|/Game/Robin/NewLevel/Blueprint/JulianUndRobin/BP_Building.BP_Building_C|GetIndex _array_element))
      (CallFunction|SetBuildingIndexonGrid _array_element (Variables|/Game/Robin/NewLevel/Blueprint/JulianUndRobin/BP_Building.BP_Building_C|GetIndex _array_element) true)
      (else
        (CallFunction|RemoveBuildingfromCombat _array_element true)))))

(fn OnTileDataUpdatet
  (params (Index :type Int%20Point%20Structure))
  (bind _output_get (LocalVariables|SetCopyOfBuildings (Variables|Default|GetBuilding)))
  (bind _array_element (Utilities|Array|ForEachLoopwithBreak _output_get :!label _label)
    (:LoopBody
      (if (Class|KismetMathLibrary|EqualIntPointIntPoint Index (Variables|/Game/Robin/NewLevel/Blueprint/JulianUndRobin/BP_Building.BP_Building_C|GetIndex _array_element))
        (if (Default|IsTileWalkable (Variables|Default|GetGrid) (Variables|/Game/Robin/NewLevel/Blueprint/JulianUndRobin/BP_Building.BP_Building_C|GetIndex _array_element))
          (CallFunction|SetBuildingIndexonGrid _array_element (Variables|/Game/Robin/NewLevel/Blueprint/JulianUndRobin/BP_Building.BP_Building_C|GetIndex _array_element) false)
          (goto _label Break)
          (else
            (CallFunction|RemoveBuildingfromCombat _array_element true)
            (goto _label Break)))))))

(fn OnUnitReachedNewTile
  (params (Building :type BP%20Building%20Object%20Reference) (Index :type Int%20Point%20Structure))
  (CallFunction|SetBuildingIndexonGrid Building Index false))