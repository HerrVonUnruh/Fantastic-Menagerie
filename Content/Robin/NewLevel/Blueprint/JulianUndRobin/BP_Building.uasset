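; BP_Building is a building actor that carries its type, data and a grid reference.
; SetBuildingData stores the data, updates the type and applies the data's static mesh, while SetGrid stores the grid.
; The construction script's default-data lookup is disconnected, as are the hover and selection setters and their ColorMultiply material tint, so those functions currently do nothing.
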(event EventBeginPlay)

(fn ConstructionScript)

(fn UpdateVisualifHoveredorSelected)

(fn SetIsHovered
  (params (Hovered :type Boolean)))

(fn SetIsSelected
  (params (Selected :type Boolean)))

(fn SetBuildingData
  (params (Data :type S%20Building%20Data%20Structure%20%28by%20ref%29))
  (bind _output_get (Variables|Default|SetBuildingData Data))
  (Variables|Default|SetBuildingType (.Type (Utilities|Struct|BreakS_BuildingData _output_get)))
  (Components|StaticMesh|SetStaticMesh (Variables|Default|GetStaticMesh) (.Mesh (Utilities|Struct|BreakS_BuildingData_Assets (.Assets (Utilities|Struct|BreakS_BuildingData _output_get))))))

(fn SetGrid
  (params (Grid :type BP%20Grid%20Object%20Reference))
  (Variables|Default|SetGrid Grid))