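; Creature character that autonomously manages hunger, thirst and sleep needs, with data from its UnitType and a material tint when selected.
; Delay-gated Tick drains needs and, by priority, sends it via AIMoveTo to the nearest BP_Trog, BP_Fountain or Place2Sleep, otherwise wandering randomly.
; Overlapping the matching actor stops movement, sets an animation state and refills that need through a looping Delay until full.
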(event Custom|IsHovered)

(event Custom|IsSelected
  (Rendering|Material|SetVectorParameterValueonMaterials (Variables|Character|GetMesh) "ColorMultiply" (Math|Conversions|ToVector(LinearColor) (* (select (Variables|Default|GetSelected) "(R=0.901927,G=0.963542,B=0.186800,A=1.000000)" "(R=1.000000,G=1.000000,B=1.000000,A=1.000000)") (select (Variables|Default|GetSelected) 2.5 1.0)))))

(event EventTick
  (params (DeltaSeconds :type Float%20%28single-precision%29))
  (bind _returnvalue (Transformation|GetActorLocation))
  (bind _randomlocation (AI|Navigation|GetRandomReachablePointinRadius _returnvalue 2e+03 0 0))
  (Utilities|FlowControl|Delay 1.0)
  (CallFunction|HungerNeed)
  (CallFunction|ThirstNeed)
  (CallFunction|SleepNeed)
  (if (Math|Boolean|ANDBoolean (!= (Variables|Default|GetIsDrinking) true) (!= (Variables|Default|GetIsSleeping) true) (Variables|Default|GetIsHungry))
    (Utilities|FlowControl|DoOnce false :!label _label
      (:Completed
        (Variables|/Script/Engine.CharacterMovementComponent|SetMaxWalkSpeed (Variables|Character|GetCharacterMovement) (.MaxWalkSpeed (Utilities|Struct|BreakS_UnitData_Assets (.Assets (Utilities|Struct|BreakS_UnitData (Variables|Default|GetUnitData))))))
        (Variables|Default|SetIsMoving true)
        (Variables|Default|SetcanMove false)
        ;[0.6667 0.09011 0.1767 1 72] Eating
        (bind _outactors (Actor|GetAllActorsOfClass "/Game/Artists/Alex/Futter_Trog/BP_Trog.BP_Trog_C"))
        (Class|BPICreatureAnimation|SetCreatureAnimationState(Message) (Components|SkeletalMesh|GetAnimInstance (Variables|Character|GetMesh)) "NewEnumerator1")
        (AI|AIMoveTo self "0, 0, 0" (.ReturnValue (Actor|FindNearestActor (Transformation|GetWorldLocation (Variables|Character|GetMesh)) _outactors)) (Math|Random|RandomFloatinRange (Variables|Default|GetSpeed) (Class|MovementComponent|GetMaxSpeed (Variables|Character|GetCharacterMovement self))) false
          (:OnSuccess
            (if (not (Variables|Default|GetIsEating))
              (goto _label Reset))))))
    (elif (Math|Boolean|ANDBoolean (!= (Variables|Default|GetIsEating) true) (!= (Variables|Default|GetIsSleeping) true) (Variables|Default|GetIsThirsty))
      (Utilities|FlowControl|DoOnce false :!label _label_2
        (:Completed
          (Variables|/Script/Engine.CharacterMovementComponent|SetMaxWalkSpeed (Variables|Character|GetCharacterMovement) (.MaxWalkSpeed (Utilities|Struct|BreakS_UnitData_Assets (.Assets (Utilities|Struct|BreakS_UnitData (Variables|Default|GetUnitData))))))
          (Variables|Default|SetIsMoving true)
          ;[0 0.6667 0.2044 1 72] Drinking
          (Variables|Default|SetcanMove false)
          (bind _outactors_2 (Actor|GetAllActorsOfClass "/Game/Artists/Alex/Water_Fountain/BP_Fountain.BP_Fountain_C"))
          (Class|BPICreatureAnimation|SetCreatureAnimationState(Message) (Components|SkeletalMesh|GetAnimInstance (Variables|Character|GetMesh)) "NewEnumerator1")
          (AI|AIMoveTo self "0, 0, 0" (.ReturnValue (Actor|FindNearestActor (Transformation|GetWorldLocation (Variables|Character|GetMesh)) _outactors_2)) (Math|Random|RandomFloatinRange (Variables|Default|GetSpeed) (Class|MovementComponent|GetMaxSpeed (Variables|Character|GetCharacterMovement self))) false
            (:OnSuccess
              (if (not (Variables|Default|GetIsDrinking))
                (goto _label_2 Reset))))))
      (elif (Math|Boolean|ANDBoolean (!= (Variables|Default|GetIsDrinking) true) (!= (Variables|Default|GetIsEating) true) (Variables|Default|GetNeeds2Sleep))
        (Utilities|FlowControl|DoOnce false :!label _label_3
          (:Completed
            ;[0.08897 0.2251 1 1 72] Sleep
            (Variables|Default|SetIsMoving true)
            (Variables|Default|SetcanMove false)
            (bind _outactors_3 (Actor|GetAllActorsOfClass "/Game/TopDown/Blueprints/Place2Sleep.Place2Sleep_C"))
            (Class|BPICreatureAnimation|SetCreatureAnimationState(Message) (Components|SkeletalMesh|GetAnimInstance (Variables|Character|GetMesh)) "NewEnumerator1")
            (AI|AIMoveTo self "0, 0, 0" (.ReturnValue (Actor|FindNearestActor (Transformation|GetWorldLocation (Variables|Character|GetMesh)) _outactors_3)) (Math|Random|RandomFloatinRange (Variables|Default|GetSpeed) (Class|MovementComponent|GetMaxSpeed (Variables|Character|GetCharacterMovement self))) false
              (:OnSuccess
                (if (not (Variables|Default|GetIsSleeping))
                  (goto _label_3 Reset))))))
        (else
          (Utilities|FlowControl|Delay (Math|Random|RandomFloatinRange 1e+01 3e+01))
          (if (not (Math|Boolean|ANDBoolean (Variables|Default|GetIsMoving) (Variables|Default|GetIsEating) (Variables|Default|GetIsDrinking) (Variables|Default|GetIsSleeping)))
            ;[1 1 1] Comment
            (Variables|/Script/Engine.CharacterMovementComponent|SetMaxWalkSpeed (Variables|Character|GetCharacterMovement) (.MaxWalkSpeed (Utilities|Struct|BreakS_UnitData_Assets (.Assets (Utilities|Struct|BreakS_UnitData (Variables|Default|GetUnitData))))))
            (if (Variables|Default|GetcanMove)
              (Variables|Default|SetIsMoving true)
              (Class|BPICreatureAnimation|SetCreatureAnimationState(Message) (Components|SkeletalMesh|GetAnimInstance (Variables|Character|GetMesh)) "NewEnumerator1")
              (AI|AIMoveTo self _randomlocation 0 (Math|Random|RandomFloatinRange (Variables|Default|GetSpeed) (Class|MovementComponent|GetMaxSpeed (Variables|Character|GetCharacterMovement self))) false
                (:then
                  (Variables|Default|SetIsMoving false))
                (:OnFail
                  (Development|PrintString "FAIL")
                  (Development|PrintString (Utilities|String|ToString(Vector) _randomlocation)))))))))))

(event Collision|EventActorBeginOverlap
  (params (OtherActor :type Actor%20Object%20Reference))
  (if (Variables|Default|GetIsHungry)
    (Utilities|Casting|CastToBP_Trog OtherActor)
    (Variables|/Script/Engine.CharacterMovementComponent|SetMaxWalkSpeed (Variables|Character|GetCharacterMovement) 0.0)
    (Class|BPICreatureAnimation|SetCreatureAnimationState(Message) (Components|SkeletalMesh|GetAnimInstance (Variables|Character|GetMesh)) "NewEnumerator6")
    (Variables|Default|SetcanMove false)
    (Variables|Default|SetIsEating true)
    (Variables|Default|SetIsMoving false)
    (if (and (Variables|Default|GetIsEating) (<= (Variables|Default|GetHunger) 1e+02))
      (Variables|Default|SetHunger (Math|Float|Clamp(Float) (+ (Variables|Default|GetHunger) 2.0) 0.0 1e+02) :!label _label)
      (if (>= (Variables|Default|GetHunger) 1e+02)
        (Variables|Default|SetIsEating false)
        (Variables|Default|SetcanMove true)
        (Class|BPICreatureAnimation|SetCreatureAnimationState(Message) (Components|SkeletalMesh|GetAnimInstance (Variables|Character|GetMesh)) "NewEnumerator0")
        (else
          (Utilities|FlowControl|Delay 1.0)
          (goto _label))))
    (elif (Variables|Default|GetIsThirsty)
      (Utilities|Casting|CastToBP_Fountain OtherActor)
      (Variables|/Script/Engine.CharacterMovementComponent|SetMaxWalkSpeed (Variables|Character|GetCharacterMovement) 0.0)
      (Class|BPICreatureAnimation|SetCreatureAnimationState(Message) (Components|SkeletalMesh|GetAnimInstance (Variables|Character|GetMesh)) "NewEnumerator6")
      (Variables|Default|SetcanMove false)
      (Variables|Default|SetIsDrinking true)
      (Variables|Default|SetIsMoving false)
      (if (and (Variables|Default|GetIsDrinking) (<= (Variables|Default|GetThirst) 1e+02))
        (Variables|Default|SetThirst (Math|Float|Clamp(Float) (+ (Variables|Default|GetThirst) 3.0) 0.0 1e+02) :!label _label_2)
        (if (>= (Variables|Default|GetThirst) 1e+02)
          (Variables|Default|SetIsDrinking false)
          (Variables|Default|SetcanMove true)
          (Class|BPICreatureAnimation|SetCreatureAnimationState(Message) (Components|SkeletalMesh|GetAnimInstance (Variables|Character|GetMesh)) "NewEnumerator0")
          (else
            (Utilities|FlowControl|Delay 1.0)
            (goto _label_2))))
      (elif (Variables|Default|GetNeeds2Sleep)
        (Utilities|Casting|CastToPlace2Sleep OtherActor)
        (Variables|/Script/Engine.CharacterMovementComponent|SetMaxWalkSpeed (Variables|Character|GetCharacterMovement) 0.0)
        (Class|BPICreatureAnimation|SetCreatureAnimationState(Message) (Components|SkeletalMesh|GetAnimInstance (Variables|Character|GetMesh)) "NewEnumerator3")
        (Variables|Default|SetcanMove false)
        (Variables|Default|SetIsSleeping true)
        (Variables|Default|SetIsMoving false)
        (if (and (Variables|Default|GetIsSleeping) (<= (Variables|Default|GetSleep) 1e+02))
          (Variables|Default|SetSleep (Math|Float|Clamp(Float) (+ (Variables|Default|GetSleep) 1.0) 0.0 1e+02) :!label _label_3)
          (if (>= (Variables|Default|GetSleep) 1e+02)
            (Variables|Default|SetIsSleeping false)
            (Variables|Default|SetcanMove true)
            (Class|BPICreatureAnimation|SetCreatureAnimationState(Message) (Components|SkeletalMesh|GetAnimInstance (Variables|Character|GetMesh)) "NewEnumerator5")
            (else
              (Utilities|FlowControl|Delay 1.0)
              (goto _label_3))))))))

(event EventBeginPlay
  (Variables|/Script/Engine.CharacterMovementComponent|SetMaxWalkSpeed (Variables|Character|GetCharacterMovement) (.MaxWalkSpeed (Utilities|Struct|BreakS_UnitData_Assets (.Assets (Utilities|Struct|BreakS_UnitData (Variables|Default|GetUnitData)))))))

(fn ConstructionScript
  (bind _unitdata (CallFunction|GetDefaultUnitDatafromUnitType (Variables|Default|GetUnitType)))
  (CallFunction|SetUnitData _unitdata))

(fn HungerNeed
  (if (Variables|Default|GetIsEating)
    _
    (else
      (bind _output_get (Variables|Default|SetHunger (Math|Float|Clamp(Float) (- (Variables|Default|GetHunger) 0.3) 0.0 1e+02)))))
  (if (<= _output_get 5e+01)
    (Variables|Default|SetIsHungry true)
    (else
      (Variables|Default|SetIsHungry false))))

(fn SleepNeed
  (if (Variables|Default|GetIsSleeping)
    _
    (else
      (bind _output_get (Variables|Default|SetSleep (Math|Float|Clamp(Float) (- (Variables|Default|GetSleep) 0.2) 0.0 1e+02)))))
  (if (<= _output_get 5e+01)
    (Variables|Default|SetNeeds2Sleep true)
    (else
      (Variables|Default|SetNeeds2Sleep false))))

(fn ThirstNeed
  (if (Variables|Default|GetIsDrinking)
    _
    (else
      (bind _output_get (Variables|Default|SetThirst (Math|Float|Clamp(Float) (- (Variables|Default|GetThirst) 0.5) 0.0 1e+02)))))
  (if (<= _output_get 5e+01)
    (Variables|Default|SetIsThirsty true)
    (else
      (Variables|Default|SetIsThirsty false))))

(fn SetUnitData
  (params (Data :type S%20Unit%20Data%20Structure%20%28by%20ref%29))
  (bind _mesh (Variables|Character|GetMesh))
  (bind _output_get (Variables|Default|SetUnitData Data))
  (if (.isAutoPossessed (Utilities|Struct|BreakS_UnitData_Assets (.Assets (Utilities|Struct|BreakS_UnitData _output_get))))
    (Variables|/Script/Engine.SkeletalMeshComponent|SetSkeletalMeshAsset _mesh (.Mesh (Utilities|Struct|BreakS_UnitData_Assets (.Assets (Utilities|Struct|BreakS_UnitData _output_get)))))
    (Class|SkeletalMeshComponent|SetAnimClass _mesh (.AnimBp (Utilities|Struct|BreakS_UnitData_Assets (.Assets (Utilities|Struct|BreakS_UnitData _output_get)))))))